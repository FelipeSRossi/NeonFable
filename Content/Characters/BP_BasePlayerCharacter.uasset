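; Base multiplayer player character for NeonFable, combining auto-attack combat with a team-versus summoning economy.
; Charged summons spend currency that accrues each second, boost income, and spawn the selected enemy type and tier around a random opposing-team pawn.
; Tick drives cooldown-limited sword attacks; XP pickups trigger Knight data-table level-ups in PlayerStruct.
; Actions route through Client/Server event pairs by authority; skill timers and the skill-point check are stubs.
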(event `ChangeSummonTypeServer`
  (params (Direction :type Boolean))
  (`self.ChangeSummonType` Direction))

(event `ResetChangingTypeCooldown`
  (set `self.ChangingTypeCooldown` false))

(event `ChangeSummonTypeClient`
  (params (Direction :type Boolean))
  (`self.ChangeSummonTypeServer` Direction))

(event `self.HandleSummonSwitchLeftCommand`
  ;[1 1 1] Summon
  (if (not (`self.ChangingTypeCooldown`))
    (set `self.ChangingTypeCooldown` true)
    (`KismetSystemLibrary.K2_SetTimerDelegate` (delegate `ResetChangingTypeCooldown`) 0.6)
    (`/Engine/EditorBlueprintResources/ActorMacros.Switch Has Authority`
      (:`Authority`
        (if (`KismetSystemLibrary.IsServer`)
          (`self.ChangeSummonTypeServer` false)
          (else
            (`self.ChangeSummonTypeClient` false :!label _label))))
      (:`Remote`
        (goto _label)))))

(event `self.HandleSummon1Command`
  ;[1 1 1] Summon
  (`/Engine/EditorBlueprintResources/ActorMacros.Switch Has Authority`
    (:`Authority`
      (if (`KismetSystemLibrary.IsServer`)
        (`self.StartSummonServer`)
        (else
          (`self.StartSummonClient` :!label _label_2))))
    (:`Remote`
      (goto _label_2))))

(event `self.HandleSummonSwitchRightCommand`
  ;[1 1 1] Summon
  (if (not (`self.ChangingTypeCooldown`))
    (set `self.ChangingTypeCooldown` true)
    (`KismetSystemLibrary.K2_SetTimerDelegate` (delegate `ResetChangingTypeCooldown`) 0.6)
    (`/Engine/EditorBlueprintResources/ActorMacros.Switch Has Authority`
      (:`Authority`
        (if (`KismetSystemLibrary.IsServer`)
          (`self.ChangeSummonTypeServer` true)
          (else
            (`self.ChangeSummonTypeClient` true :!label _label_3))))
      (:`Remote`
        (goto _label_3)))))

(event `self.HandleSummon1ReleaseCommand`
  ;[1 1 1] Summon
  (`/Engine/EditorBlueprintResources/ActorMacros.Switch Has Authority`
    (:`Authority`
      (if (`KismetSystemLibrary.IsServer`)
        (`self.SummonEnemyServer`)
        (else
          (`self.SummonEnemyClient` :!label _label_4))))
    (:`Remote`
      (goto _label_4))))

(event `SummonLocationClient`
  ;[1 1 1] Summon
  (`self.SummonLocationServer`))

(event `SummonLocationServer`
  ;[1 1 1] Summon
  (`self.SummonLocationSelect`))

(event `DecreaseCURIncreaseINC_SERVER`
  (bind (_player_struct_hp _player_struct_hp_max _player_struct_cur _player_struct_inc) (break `/Game/Characters/Player_Data_Struct` (`self.Player_Struct`)))
  ;[1 1 1] Summon
  (bind _parameterresponse (`self.GetEnemyDataFromStruct` "INC_VALUE"))
  (setmembers `/Game/Characters/Player_Data_Struct` :`StructRef` (`self.Player_Struct`) :`CUR` (- _player_struct_cur (* (`self.SummonLvl`) 100)) :`INC` (+ _parameterresponse _player_struct_inc)))

(event `DecreaseCURIncreaseINC_CLIENT`
  ;[1 1 1] Summon
  (`self.DecreaseCURIncreaseINC_SERVER`))

(event `SummonEnemyClient`
  ;[1 1 1] Summon
  (`self.SummonEnemyServer`))

(event `SummonEnemyServer`
  (bind (_player_struct_hp _player_struct_hp_max _player_struct_cur _player_struct_inc) (break `/Game/Characters/Player_Data_Struct` (`self.Player_Struct`)))
  ;[1 1 1] Summon
  (`self.SetSummonLvl`)
  (if (`self.IsSummonCooldown`)
    _
    (elif (and (>= (`self.SummonCharge`) 100) (>= _player_struct_cur 100))
      (set `self.IsSummoning` false)
      (set `self.IsSummoningSuccessful` true)
      (set `self.SummonCharge` 0)
      (`self.ActivateCylinderParticleMulticast`)
      (`/Engine/EditorBlueprintResources/ActorMacros.Switch Has Authority`
        (:`Authority`
          (if (`KismetSystemLibrary.IsServer`)
            (`self.DecreaseCURIncreaseINC_SERVER`)
            (`self.SummonLocationServer`)
            (else
              (`self.DecreaseCURIncreaseINC_CLIENT` :!label _label_5)
              (`self.SummonLocationClient`))))
        (:`Remote`
          (goto _label_5)))
      (`self.SetSummonLvl`)
      (else
        (set `self.IsSummoning` false)
        (set `self.IsSummoningSuccessful` false)
        (set `self.SummonCharge` 0)))))

(event `StartSummonClient`
  ;[1 1 1] Summon
  (`self.StartSummonServer`))

(event `ActivateCylinderParticleMulticast`
  ;[1 1 1] Summon
  (`NiagaraFunctionLibrary.SpawnSystemAttached` "/Game/Particles/NS_Cylinder.NS_Cylinder" (`self.Mesh`) "None" (0.0 0.0 -100.0) (struct) "KeepRelativeOffset"))

(event `StartSummonServer`
  ;[1 1 1] Summon
  (set `self.IsSummoningSuccessful` false)
  (set `self.SummonCharge` (+ (`self.SummonCharge`) 1))
  (set `self.IsSummoning` true)
  (`self.SetSummonLvl`))

(event `AddIncome`
  (bind (_player_struct_hp _player_struct_hp_max _player_struct_cur _player_struct_inc) (break `/Game/Characters/Player_Data_Struct` (`self.Player_Struct`)))
  ;[1 1 1] Begin Play
  (setmembers `/Game/Characters/Player_Data_Struct` :`StructRef` (`self.Player_Struct`) :`CUR` (+ _player_struct_cur _player_struct_inc)))

(event `self.ReceiveBeginPlay`
  (bind (_player_struct_hp _player_struct_hp_max _player_struct_cur _player_struct_inc _player_struct_lvl _player_struct_xp _player_struct_atk _player_struct_atk_spd _player_struct_mv_spd) (break `/Game/Characters/Player_Data_Struct` (`self.Player_Struct`)))
  ;[1 1 1] Begin Play
  (set `CharacterMovementComponent.MaxWalkSpeed` (+ (* (`KismetMathLibrary.Conv_IntToDouble` _player_struct_mv_spd) 1.0) 500.0) (`self.CharacterMovement`))
  (if (`KismetSystemLibrary.IsServer`)
    (bind _asbp_neon_fable_game_mode_mp (cast `/Game/GameMode/BP_NeonFableGameModeMP` (`GameplayStatics.GetGameMode`)))
    (set `self.GameMode` _asbp_neon_fable_game_mode_mp)
    (`KismetSystemLibrary.K2_SetTimerDelegate` (delegate `AddIncome`) 1.0 true)))

(event `self.BasicAttackCollision.OnComponentBeginOverlap`
  (params (OverlappedComponent :type "PrimitiveComponent Object Reference") (OtherActor :type "Actor Object Reference") (OtherComp :type "PrimitiveComponent Object Reference") (OtherBodyIndex :type Integer) (bFromSweep :type Boolean) (SweepResult :type "HitResult Structure (by ref)"))
  ;[1 1 1] Weapon Collision
  (if (!= (`GameplayStatics.GetObjectClass` OtherActor) (`GameplayStatics.GetObjectClass` self))
    (`/Engine/EditorBlueprintResources/ActorMacros.Switch Has Authority`
      (:`Authority`
        (if (`KismetSystemLibrary.IsServer`)
          (`self.ApplyDamageClient` OtherActor)
          (else
            (`self.ApplyDamageServer` OtherActor :!label _label_6))))
      (:`Remote`
        (goto _label_6)))))

(event `Set GameInstance`
  (params (GameInstance :type Integer))
  (set `self.GameInstance` GameInstance))

(event `self.ReceiveTick`
  (params (DeltaSeconds :type "Float (single-precision)"))
  ;[1 1 1] Event Tick
  (if (not (`self.IsBasicAttackOnCooldown`))
    (`/Engine/EditorBlueprintResources/ActorMacros.Switch Has Authority`
      (:`Authority`
        (if (`KismetSystemLibrary.IsServer`)
          (`self.HandleBasicAttackCommandServer`)
          (else
            (`self.HandleBasicAttackCommandClient` :!label _label_7))))
      (:`Remote`
        (goto _label_7)))))

(event `HandleBasicAttackCommandClient`
  ;[1 1 1] Handle Basic Attack
  (`self.HandleBasicAttackCommandServer`))

(event `self.HandleRotation`
  (params (Rotation :type "Rotator Structure (by ref)"))
  ;[1 1 1] Rotation
  (`self.SetRotationServer` Rotation))

(event `self.HandleBasicAttackCommand`
  ;[1 1 1] Handle Basic Attack
)

(event `HandleBasicAttackCommandServer`
  ;[1 1 1] Handle Basic Attack
  (if (and (not (`self.IsBasicAttacking`)) (not (`self.IsBasicAttackOnCooldown`)))
    (set `self.IsBasicAttacking` true)))

(event `SetRotationServer`
  (params (Rotation :type "Rotator Structure"))
  ;[1 1 1] Rotation
  (bind _output_get (set `self.ServerRotation` Rotation))
  (if (`self.CanRotate`)
    (`self.K2_SetActorRotation` _output_get)
    (`self.SetRotationClient` _output_get)))

(event `Basic Attack Command Slash Arc Start`
  ;[1 1 1] Particles
  (`self.AttackRibbonActivate`)
  (`self.AttackRibbonServer`)
  (set `PrimitiveComponent.bGenerateOverlapEvents` true (`self.BasicAttackCollision`)))

(event `ApplyDamageClient`
  (params (EnemyToDamage :type "Actor Object Reference"))
  ;[1 1 1] Deal Damage
  (`self.ApplyDamageServer` EnemyToDamage))

(event `AttackRibbonServer`
  ;[1 1 1] Particles
  (`self.AttackRibbonActivate`))

(event `AttackRibbonActivate`
  ;[1 1 1] Particles
  (bind _returnvalue (`NiagaraFunctionLibrary.SpawnSystemAttached` "/Game/Particles/NS_SwordRibbon.NS_SwordRibbon" (`self.Sword`) "None" (-14.0 -40.0 100.0) (struct) "KeepRelativeOffset"))
  (set `self.SwordRibbon` _returnvalue))

(event `ApplyDamageServer`
  (params (EnemyToDamage :type "Actor Object Reference"))
  (bind (_player_struct_hp _player_struct_hp_max _player_struct_cur _player_struct_inc _player_struct_lvl _player_struct_xp _player_struct_atk) (break `/Game/Characters/Player_Data_Struct` (`self.Player_Struct`)))
  ;[1 1 1] Deal Damage
  (`GameplayStatics.ApplyDamage` EnemyToDamage (`KismetMathLibrary.Conv_IntToDouble` _player_struct_atk) null self "/Game/Characters/BP_BasicAttackDamageType.BP_BasicAttackDamageType_C"))

(event `Basic Attack Command Slash Arc End`
  ;[1 1 1] Particles
  (`self.AttackRibbonDeactivateMulticast`))

(event `Basic Attack Command Animation Finished`
  ;[1 1 1] Handle Basic Attack
  (`/Engine/EditorBlueprintResources/ActorMacros.Switch Has Authority`
    (:`Authority`
      (if (`KismetSystemLibrary.IsServer`)
        (`self.BasicAttackFinishedServer`)
        (else
          (`self.BasicAttackFinishedClient` :!label _label_8))))
    (:`Remote`
      (goto _label_8))))

(event `SetRotationClient`
  (params (Rotation :type "Rotator Structure"))
  ;[1 1 1] Rotation
  (if (`self.CanRotate`)
    (`self.K2_SetActorRotation` Rotation)))

(event `AttackRibbonDeactivateMulticast`
  ;[1 1 1] Particles
)

(event `SummonLoopParticle`
  ;[1 1 1] Particles
  (`/Engine/EditorBlueprintResources/ActorMacros.Switch Has Authority`
    (:`Authority`
      (if (`KismetSystemLibrary.IsServer`)
        (`self.SummonLoopParticleServer`)
        (else
          (`self.SummonLoopParticleClient` :!label _label_9))))
    (:`Remote`
      (goto _label_9))))

(event `BasicAttackFinishedClient`
  ;[1 1 1] Handle Basic Attack
  (set `PrimitiveComponent.bGenerateOverlapEvents` false (`self.BasicAttackCollision`))
  (`self.BasicAttackFinishedServer`))

(event `StartBasicAttackCommandCooldown`
  (bind (_player_struct_hp _player_struct_hp_max _player_struct_cur _player_struct_inc _player_struct_lvl _player_struct_xp _player_struct_atk _player_struct_atk_spd) (break `/Game/Characters/Player_Data_Struct` (`self.Player_Struct`)))
  ;[1 1 1] Handle Basic Attack
  (set `self.IsBasicAttackOnCooldown` true)
  (`KismetSystemLibrary.K2_SetTimerDelegate` (delegate `OnBasicAttackCooldownEnd`) (/ 10.0 (`KismetMathLibrary.Conv_IntToDouble` _player_struct_atk_spd))))

(event `BasicAttackFinishedServer`
  ;[1 1 1] Handle Basic Attack
  (set `self.IsBasicAttacking` false)
  (set `PrimitiveComponent.bGenerateOverlapEvents` false (`self.BasicAttackCollision`))
  (`self.StartBasicAttackCommandCooldown`))

(event `SummonLoopParticleClient`
  ;[1 1 1] Particles
  (`self.SummonLoopParticleServer`))

(event `OnBasicAttackCooldownEnd`
  ;[1 1 1] Handle Basic Attack
  (set `self.IsBasicAttackOnCooldown` false))

(event `SummonLoopParticleServer`
  ;[1 1 1] Particles
  (`self.SummonLoopMulticast`))

(event `SummonLoopMulticast`
  ;[1 1 1] Particles
  (`self.ActivateSummonParticle`))

(event `self.HandleSkill1LevelUp`
  (`/Engine/EditorBlueprintResources/ActorMacros.Switch Has Authority`
    (:`Authority`
      (if (`KismetSystemLibrary.IsServer`)
        (`self.Handle Skill Level Up Server` 1)
        (else
          (`self.Handle Skill Level Up Client` 1 :!label _label_10))))
    (:`Remote`
      (goto _label_10))))

(event `CollectConsumable`
  (params (ConsumableName :type String))
  (bind (_player_struct_hp _player_struct_hp_max _player_struct_cur _player_struct_inc _player_struct_lvl _player_struct_xp) (break `/Game/Characters/Player_Data_Struct` (`self.Player_Struct`)))
  ;[1 1 1] Consumable
  (switch `string` ConsumableName
    (:`XP1`
      (setmembers `/Game/Characters/Player_Data_Struct` :`StructRef` (`self.Player_Struct`) :`XP` (+ _player_struct_xp 100))
      (`/Engine/EditorBlueprintResources/ActorMacros.Switch Has Authority`
        (:`Authority`
          (if (`KismetSystemLibrary.IsServer`)
            (`self.AbsorbOrb_SERVER`)
            (`self.LevelUpServer`)
            (else
              (`self.AbsorbOrb_CLIENT` :!label _label_11)
              (`self.LevelUpClient`))))
        (:`Remote`
          (goto _label_11))))))

(event `self.HandleLevelUpMode`
  (`KismetSystemLibrary.PrintString` "Hello"))

(event `self.ReceiveAnyDamage`
  (params (Damage :type "Float (single-precision)") (DamageType :type "DamageType Object Reference") (InstigatedBy :type "Controller Object Reference") (DamageCauser :type "Actor Object Reference"))
  (bind _player_struct_hp (break `/Game/Characters/Player_Data_Struct` (`self.Player_Struct`)))
  ;[1 1 1] Receive Damage
  (`/Engine/EditorBlueprintResources/ActorMacros.Switch Has Authority`
    (:`Authority`
      (bind _structout (setmembers `/Game/Characters/Player_Data_Struct` :`StructRef` (stale _output_get) :`HP` (`KismetMathLibrary.FTrunc` (- _player_struct_hp Damage))))
      (bind _output_get (set `self.Player_Struct` _structout))
      (if (`KismetSystemLibrary.IsServer`)
        (`self.DamageFlash_SERVER`)
        (else
          (`self.DamageFlash_CLIENT`))))))

(event `Handle Skill Level Up Client`
  (params (`Skill Number` :type Integer))
  (`self.Handle Skill Level Up Server` `Skill Number`))

(event `LevelUpClient`
  ;[1 1 1] Consumable
  (`self.LevelUpServer`))

(event `LevelUpServer`
  ;[1 1 1] Consumable
  (`self.LevelUp`))

(event `Handle Skill Level Up Server`
  (params (`Skill number` :type Integer))
  (bind (_player_struct_hp _player_struct_hp_max _player_struct_cur _player_struct_inc _player_struct_lvl _player_struct_xp _player_struct_atk _player_struct_atk_spd _player_struct_mv_spd _player_struct_atk_size _player_struct_class _player_struct_cdr _player_struct_skill_power _player_struct_xp_to_lvl _player_struct_skill1_lvl _player_struct_skill2_lvl _player_struct_skill3_lvl _player_struct_skill4_lvl _player_struct_skill_points) (break `/Game/Characters/Player_Data_Struct` (`self.Player_Struct`)))
  (bind _player_struct (`self.Player_Struct`))
  (bind _returnvalue (- _player_struct_skill_points 1))
  (bind _return (`self.CheckIfCanLevelSkillUp` `Skill number` _player_struct_skill_points))
  (if _return
    (switch `int` `Skill number`
      (:`1`
        (setmembers `/Game/Characters/Player_Data_Struct` :`StructRef` _player_struct :`SKILL1_LVL` (+ _player_struct_skill1_lvl 1) :`SKILL_POINTS` _returnvalue))
      (:`2`
        (setmembers `/Game/Characters/Player_Data_Struct` :`StructRef` _player_struct :`SKILL2_LVL` (+ _player_struct_skill2_lvl 1) :`SKILL_POINTS` _returnvalue))
      (:`3`
        (setmembers `/Game/Characters/Player_Data_Struct` :`StructRef` _player_struct :`SKILL3_LVL` (+ _player_struct_skill3_lvl 1) :`SKILL_POINTS` _returnvalue))
      (:`4`
        (setmembers `/Game/Characters/Player_Data_Struct` :`StructRef` _player_struct :`SKILL4_LVL` (+ _player_struct_skill4_lvl 1) :`SKILL_POINTS` _returnvalue)))))

(event `ActivateLVLUpParticleMulticast`
  ;[1 1 1] Consumable
  (`NiagaraFunctionLibrary.SpawnSystemAttached` "/Game/Particles/NS_Cylinder_LVLUP.NS_Cylinder_LVLUP" (`self.CapsuleComponent`) "None" (0.0 0.0 0.0) (struct) "KeepRelativeOffset"))

(event `DamageFlash_CLIENT`
  ;[1 1 1] Receive Damage
  (`self.DamageFlash_SERVER`))

(event `AbsorbOrb_CLIENT`
  ;[1 1 1] Consumable
  (`self.AbsorbOrb_SERVER`))

(event `DamageFlash_SERVER`
  ;[1 1 1] Receive Damage
  (bind _returnvalue (`PrimitiveComponent.CreateDynamicMaterialInstance` (`self.Mesh`) 0 "/Game/Characters/Knight/Materials/NewKnight_Material_Player_Inst.NewKnight_Material_Player_Inst" "None"))
  (bind (_direction _newtrack_1) (`Timeline|Timeline` :!via `PlayFromStart`)
    (:`Update`
      (`MaterialInstanceDynamic.SetScalarParameterValue` _returnvalue "Contrast" _newtrack_1))
    (:`Finished`
      (`MaterialInstanceDynamic.SetScalarParameterValue` _returnvalue "Contrast" 1.0)))
  (`PrimitiveComponent.SetMaterial` (`self.Mesh`) 0 _returnvalue))

(event `AbsorbOrb_SERVER`
  ;[1 1 1] Consumable
  (`NiagaraFunctionLibrary.SpawnSystemAttached` "/Game/Particles/NS_Explosion_Custom-2.NS_Explosion_Custom-2" (`self.Mesh`) "None" (0.0 0.0 100.0) (struct) "KeepRelativeOffset"))

(fn `ActivateSummonParticle`
  (if (== (`self.SummonLvl`) 0)
    (if (`self.HasSummonLoopParticle`)
      (if (not (`ActorComponent.IsActive` (`self.SummonLoopParticleEffect`)))
        (bind _returnvalue (`NiagaraFunctionLibrary.SpawnSystemAttached` "/Game/Particles/NS_Summon_Energy_Lvl0.NS_Summon_Energy_Lvl0" (`self.CapsuleComponent`) "None" (0.0 0.0 0.0) (struct) "KeepRelativeOffset" :!label _label))
        (set `self.SummonLoopParticleEffect` _returnvalue)
        (set `self.HasSummonLoopParticle` true)
        (return))
      (else
        (goto _label)))
    (elif (== (`self.SummonLvl`) 1)
      (if (`self.HasSummonLoopParticle`)
        (if (not (`ActorComponent.IsActive` (`self.SummonLoopParticleEffect`)))
          (bind _returnvalue_2 (`NiagaraFunctionLibrary.SpawnSystemAttached` "/Game/Particles/NS_Summon_Energy_Lvl1.NS_Summon_Energy_Lvl1" (`self.CapsuleComponent`) "None" (0.0 0.0 0.0) (struct) "KeepRelativeOffset" :!label _label_2))
          (set `self.SummonLoopParticleEffect` _returnvalue_2)
          (set `self.HasSummonLoopParticle` true)
          (return))
        (else
          (goto _label_2)))
      (elif (== (`self.SummonLvl`) 2)
        (if (`self.HasSummonLoopParticle`)
          (if (not (`ActorComponent.IsActive` (`self.SummonLoopParticleEffect`)))
            (bind _returnvalue_3 (`NiagaraFunctionLibrary.SpawnSystemAttached` "/Game/Particles/NS_Summon_Energy_Lvl2.NS_Summon_Energy_Lvl2" (`self.CapsuleComponent`) "None" (0.0 0.0 0.0) (struct) "KeepRelativeOffset" :!label _label_3))
            (set `self.SummonLoopParticleEffect` _returnvalue_3)
            (set `self.HasSummonLoopParticle` true)
            (return))
          (else
            (goto _label_3)))
        (else
          (return))))))

(fn `ChangeSummonType`
  (params (Direction :type Boolean))
  (if Direction
    (switch `string` (`self.SummonType`)
      (:`CONE_`
        (set `self.SummonType` "SPHERE_" :!label _label))
      (:`OCTA_`
        (set `self.SummonType` "CONE_" :!label _label_2))
      (:`CUBE_`
        (set `self.SummonType` "OCTA_" :!label _label_3))
      (:`SPHERE_`
        (set `self.SummonType` "CUBE_" :!label _label_4)))
    (else
      (switch `string` (`self.SummonType`)
        (:`CONE_`
          (goto _label_3))
        (:`OCTA_`
          (goto _label_4))
        (:`CUBE_`
          (goto _label))
        (:`SPHERE_`
          (goto _label_2))))))

(fn `CheckIfCanLevelSkillUp`
  (params (`Skill Number` :type Integer) (`Skill Points` :type Integer))
  (returns (Return :type Boolean))
  (return true))

(fn `GetEnemyClass`
  (returns (ParameterResponse :type "/Game/Enemies/BaseEnemyBlueprint Class Reference"))
  (switch `string` (`KismetStringLibrary.Concat_StrStr` (`self.SummonType`) (`KismetStringLibrary.Conv_IntToString` (`self.SummonLvl`)))
    (:`CONE_1`
      (return "/Game/Enemies/ConeTier1/ConeTier1Blueprint.ConeTier1Blueprint_C"))
    (:`CONE_2`
      (return "/Game/Enemies/ConeTier2/ConeTier2Blueprint.ConeTier2Blueprint_C"))
    (:`CONE_3`
      (return null))
    (:`OCTA_1`
      (return "/Game/Enemies/OctaTier1/OctaTier1Blueprint.OctaTier1Blueprint_C"))))

(fn `GetEnemyDataFromStruct`
  (params (Parameter :type String))
  (returns (ParameterResponse :type Integer))
  (bind (_enemies_struct_cone_1 _enemies_struct_cone_2 _enemies_struct_cone_3 _enemies_struct_octa_1) (break `/Game/Characters/Enemies_Data_Struct` (`self.Enemies_Struct`)))
  (switch `string` (`KismetStringLibrary.Concat_StrStr` (`self.SummonType`) (`KismetStringLibrary.Conv_IntToString` (`self.SummonLvl`)))
    (:`CONE_1`
      (return (`BlueprintMapLibrary.Map_Find` _enemies_struct_cone_1 Parameter)))
    (:`CONE_2`
      (return (`BlueprintMapLibrary.Map_Find` _enemies_struct_cone_2 Parameter)))
    (:`CONE_3`
      (return (`BlueprintMapLibrary.Map_Find` _enemies_struct_cone_3 Parameter)))
    (:`OCTA_1`
      (return (`BlueprintMapLibrary.Map_Find` _enemies_struct_octa_1 Parameter)))))

(fn `LevelUp`
  (locals (NewLocalVar :type "/Game/Characters/Player_Data_Struct Structure"))
  (bind (_player_struct_hp _player_struct_hp_max _player_struct_cur _player_struct_inc _player_struct_lvl _player_struct_xp _player_struct_atk _player_struct_atk_spd _player_struct_mv_spd _player_struct_atk_size _player_struct_class _player_struct_cdr _player_struct_skill_power _player_struct_xp_to_lvl) (break `/Game/Characters/Player_Data_Struct` (`self.Player_Struct`)))
  (bind _returnvalue (`|GetDataTableRow` "/Game/Characters/ClassGrowthDataTable.ClassGrowthDataTable" "Knight")
    (:`then`
      (if (>= _player_struct_xp _player_struct_xp_to_lvl)
        (bind _returnvalue_2 (+ _player_struct_hp_max (`.HP_MAX_43_FE084EC945C0AB8A787421A413B94591` (break `/Game/Characters/Player_Data_Struct` _returnvalue))))
        (setmembers `/Game/Characters/Player_Data_Struct` :`StructRef` (`self.Player_Struct`) :`HP` (+ _player_struct_hp (- _returnvalue_2 _player_struct_hp_max)) :`HP_MAX` _returnvalue_2 :`LVL` (+ _player_struct_lvl 1) :`XP` (- _player_struct_xp _player_struct_xp_to_lvl) :`ATK` (+ _player_struct_atk (`.ATK_33_3711404E443825F6D95374B8E9CD7D21` (break `/Game/Characters/Player_Data_Struct` _returnvalue))) :`ATK_SPD` (+ _player_struct_atk_spd (`.ATK_SPD_34_A99DC2934136A90B3ACE8B92A5988840` (break `/Game/Characters/Player_Data_Struct` _returnvalue))) :`MV_SPD` (+ _player_struct_mv_spd (`.MV_SPD_35_EA5312C94D96D5B423A17D9DB54863D6` (break `/Game/Characters/Player_Data_Struct` _returnvalue))) :`ATK_SIZE` (+ _player_struct_atk_size (`.ATK_SIZE_36_0802BB794EA65827579BD89F3B06AADA` (break `/Game/Characters/Player_Data_Struct` _returnvalue))) :`CDR` (+ _player_struct_cdr (`.CDR_37_2A38DBF94A76E0BD3AE98BBBB692D6B5` (break `/Game/Characters/Player_Data_Struct` _returnvalue))) :`Skill_Power` (+ _player_struct_skill_power (`.Skill_Power_23_6C798AC64C520ED41530918727F1D40D` (break `/Game/Characters/Player_Data_Struct` _returnvalue))) :`XP_TO_LVL` (`KismetMathLibrary.FTrunc` (* (`KismetMathLibrary.Conv_IntToDouble` _player_struct_xp_to_lvl) 1.25)))
        (`self.ActivateLVLUpParticleMulticast`)
        (return)))))

(fn `OnRep_IsBasicAttacking`)

(fn `OnRep_Player_Struct`)

(fn `OnRep_Skill1Timer`
  (`self.StartLocalSkill1Timer`))

(fn `OnRep_Skill2Timer`
  (`self.StartLocalSkill2Timer`))

(fn `OnRep_Skill3Timer`
  (`self.StartLocalSkil3Timer`))

(fn `OnRep_Skill4Timer`
  (`self.StartLocalSkil4Timer`))

(fn `SetSummonLvl`
  (bind (_player_struct_hp _player_struct_hp_max _player_struct_cur) (break `/Game/Characters/Player_Data_Struct` (`self.Player_Struct`)))
  (set `self.SummonLvl` 0)
  (if (and (>= (`self.SummonCharge`) 100) (>= _player_struct_cur 100))
    (set `self.SummonLvl` 1)
    (if (and (>= (`self.SummonCharge`) 200) (>= _player_struct_cur 200))
      (set `self.SummonLvl` 2)
      (return)
      (else
        (return)))
    (else
      (return))))

(fn `StartLocalSkil3Timer`)

(fn `StartLocalSkil4Timer`)

(fn `StartLocalSkill1Timer`)

(fn `StartLocalSkill2Timer`)

(fn `SummonCooldownOff`
  (set `self.IsSummonCooldown` false))

(fn `SummonEnemy`
  (params (SummonClass :type "/Game/Enemies/BaseEnemyBlueprint Class Reference") (SummonAmount :type Integer))
  (bind (_returnvalue_x _returnvalue_y) (`KismetMathLibrary.BreakVector` (`KismetMathLibrary.RandomUnitVector`)))
  (for _ (range 1 (+ SummonAmount 1))
    (`|SpawnActorFromClass` SummonClass (`KismetMathLibrary.Conv_VectorToTransform` (+ (`self.K2_GetActorLocation` self) (* (`KismetMathLibrary.MakeVector` _returnvalue_x _returnvalue_y) (`KismetMathLibrary.RandomFloatInRange` 1000.0 2000.0)))) "Undefined" "OverrideRootScale" null (`self.GameInstance`) self null)))

(fn `SummonLocationSelect`
  (bind _gamemode (`self.GameMode`))
  (bind (_player_struct_hp _player_struct_hp_max _player_struct_cur _player_struct_inc) (break `/Game/Characters/Player_Data_Struct` (`self.Player_Struct`)))
  (bind _gamecontroller (`/Game/GameMode/BP_NeonFableGameModeMP.GameController` _gamemode))
  (bind _team1pawns (`/Game/GameMode/BP_NeonFableGameControllerMP.Team1Pawns` _gamecontroller))
  (bind _team2pawns (`/Game/GameMode/BP_NeonFableGameControllerMP.Team2Pawns` _gamecontroller))
  (bind _found (`/Game/GameMode/BP_NeonFableGameModeMP.GetGameController` _gamemode))
  (if _found
    (bind _asbp_neon_fable_game_instance_mp (cast `/Game/GameMode/BP_NeonFableGameInstanceMP` (`GameplayStatics.GetGameInstance`)))
    (`/Game/GameMode/BP_NeonFableGameInstanceMP.GetTeamNumber` _asbp_neon_fable_game_instance_mp)
    (bind _parameterresponse (`self.GetEnemyDataFromStruct` "SPAWN_NUMBER"))
    (bind _parameterresponse_2 (`self.GetEnemyDataFromStruct` "INC_VALUE"))
    (setmembers `/Game/Characters/Player_Data_Struct` :`StructRef` (`self.Player_Struct`) :`INC` (+ _parameterresponse_2 _player_struct_inc))
    (bind _parameterresponse_3 (`self.GetEnemyClass`))
    (if (== (`self.TeamNumber`) 0)
      (`self.SummonEnemy` (`|GetArrayItem` _team2pawns (`KismetMathLibrary.RandomInteger` (`KismetArrayLibrary.Array_Length` _team2pawns))) _parameterresponse_3 _parameterresponse)
      (else
        (`self.SummonEnemy` (`|GetArrayItem` _team1pawns (`KismetMathLibrary.RandomInteger` (`KismetArrayLibrary.Array_Length` _team1pawns))) _parameterresponse_3 _parameterresponse)))
    (set `self.IsSummonCooldown` true)
    (`KismetSystemLibrary.K2_SetTimer` null "SummonCooldownOff" 0.5)))

(fn `UserConstructionScript`)