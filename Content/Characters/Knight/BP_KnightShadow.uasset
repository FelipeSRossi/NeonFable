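; BP_KnightShadow is a short-lived shadow actor that performs an air slash for the instigating Knight character.
; It plays the slash at a rate scaled by the owner's attack speed, matches the owner's mesh rotation, and destroys itself when the animation ends.
; Past a set animation time, Tick enables weapon overlaps and spawns a sword ribbon each frame.
; Overlaps with other classes route damage through the owner's client or server function.
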(event `self.BasicAttackCollision.OnComponentBeginOverlap`
  (params (OverlappedComponent :type "PrimitiveComponent Object Reference") (OtherActor :type "Actor Object Reference") (OtherComp :type "PrimitiveComponent Object Reference") (OtherBodyIndex :type Integer) (bFromSweep :type Boolean) (SweepResult :type "HitResult Structure (by ref)"))
  (bind _instigatorplayer (`self.InstigatorPlayer`))
  ;[1 1 1] Weapon Collision
  (if (!= (`GameplayStatics.GetObjectClass` OtherActor) (`GameplayStatics.GetObjectClass` (`self.InstigatorPlayer`)))
    (`/Engine/EditorBlueprintResources/ActorMacros.Switch Has Authority`
      (:`Authority`
        (if (`KismetSystemLibrary.IsServer`)
          (`/Game/Characters/BP_BasePlayerCharacter.ApplyDamageClient` _instigatorplayer OtherActor)
          (else
            (`/Game/Characters/BP_BasePlayerCharacter.ApplyDamageServer` _instigatorplayer OtherActor :!label _label))))
      (:`Remote`
        (goto _label)))))

(event `self.ReceiveBeginPlay`
  (bind _knight (`self.Knight`))
  (bind _asbp_knight_character (cast `/Game/Characters/Knight/BP_KnightCharacter` (`self.GetInstigator`)))
  (set `self.InstigatorPlayer` _asbp_knight_character)
  (bind (_player_struct_hp _player_struct_hp_max _player_struct_cur _player_struct_inc _player_struct_lvl _player_struct_xp _player_struct_atk _player_struct_atk_spd) (break `/Game/Characters/Player_Data_Struct` (`/Game/Characters/BP_BasePlayerCharacter.Player_Struct` _asbp_knight_character)))
  (bind _output_get (set `self.AtkSpd` (+ (* (`KismetMathLibrary.Conv_IntToDouble` _player_struct_atk_spd) 0.00115) 1.0)))
  (`SkeletalMeshComponent.SetPlayRate` _knight _output_get)
  (`SkeletalMeshComponent.PlayAnimation` _knight "/Game/Characters/Knight/Animations/Anim2_rig_Air_Slash.Anim2_rig_Air_Slash" false))

(event `self.ReceiveTick`
  (params (DeltaSeconds :type "Float (single-precision)"))
  (bind _knight (`self.Knight`))
  (bind _basicattackcollision (`self.BasicAttackCollision`))
  (`self.K2_SetActorRotation` self (`SceneComponent.K2_GetComponentRotation` (`Character.Mesh` (`self.InstigatorPlayer`))) false)
  (if (`SkeletalMeshComponent.IsPlaying` _knight)
    (if (>= (`SkeletalMeshComponent.GetPosition` _knight) 0.388)
      (set `PrimitiveComponent.bGenerateOverlapEvents` true _basicattackcollision)
      (`self.AttackRibbonActivate`)
      (else
        (set `PrimitiveComponent.bGenerateOverlapEvents` false _basicattackcollision)))
    (else
      (`self.K2_DestroyActor`))))

(event `AttackRibbonActivate`
  (bind _returnvalue (`NiagaraFunctionLibrary.SpawnSystemAttached` "/Game/Particles/NS_SwordRibbon.NS_SwordRibbon" (`self.Sword`) "None" (-14.0 -40.0 100.0) (struct) "KeepRelativeOffset"))
  (set `self.Sword Ribbon` _returnvalue))

(fn `UserConstructionScript`)