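; Knight player character whose first skill is a sword dash; skills 2 to 4 only print placeholder text.
; The authority-side dash locks input, boosts walk speed and uses a timeline to force forward movement, with multicasts for sword pose and input state.
; A constantly spinning cone has overlaps enabled during the dash and passes non-Knight actors to damage events.
; Dash cooldown timers shorten with the CDR stat.
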(event `MulticastDisableMoveInput`
  (bind _returnvalue (`self.GetLocalViewingPlayerController`))
  (`SceneComponent.SetVisibility` (`self.Knight_Skill1_Cone`) true true)
  (`/Engine/EditorBlueprintResources/StandardMacros.IsValid` _returnvalue
    (:`Is Valid`
      (`Controller.SetIgnoreMoveInput` _returnvalue true))))

(event `MulticastEnableMoveInput`
  (bind _returnvalue (`self.GetLocalViewingPlayerController`))
  (`SceneComponent.SetVisibility` (`self.Knight_Skill1_Cone`) true true)
  (`/Engine/EditorBlueprintResources/StandardMacros.IsValid` _returnvalue
    (:`Is Valid`
      (`Controller.SetIgnoreMoveInput` _returnvalue false)
      (set `self.CanRotate` true))))

(event `MulticastSwordDashTransform`
  (params (NewTransform :type "Transform Structure"))
  (`SceneComponent.K2_SetRelativeTransform` (`self.Sword`) NewTransform true false))

(event `Handle Skill1Command Server`
  (bind _returnvalue (`self.GetLocalViewingPlayerController`))
  (bind _returnvalue_2 (`self.GetLocalViewingPlayerController`))
  (bind _charactermovement (`self.CharacterMovement`))
  (bind _knight_skill1_cone (`self.Knight_Skill1_Cone`))
  (bind (_player_struct_hp _player_struct_hp_max _player_struct_cur _player_struct_inc _player_struct_lvl _player_struct_xp _player_struct_atk _player_struct_atk_spd _player_struct_mv_spd) (break `/Game/Characters/Player_Data_Struct` (`self.Player_Struct`)))
  (bind _knight_skill1_cone_2 (`self.Knight_Skill1_Cone`))
  (`/Engine/EditorBlueprintResources/ActorMacros.Switch Has Authority`
    (:`Authority`
      (if (not (or (`self.IsDashOnCooldown`) (`self.IsDashing`)))
        (`/Engine/EditorBlueprintResources/StandardMacros.IsValid` _returnvalue
          (:`Is Valid`
            (`Controller.SetIgnoreMoveInput` _returnvalue true))
          (:`Is Not Valid`
            _))
        (set `self.IsDashing` true)
        (set `self.CanRotate` false)
        (set `self.DashDirection` (`self.GetActorForwardVector`))
        (set `CharacterMovementComponent.MaxWalkSpeed` 4500.0 _charactermovement)
        (`self.MulticastSwordDashTransform` (`self.SwordDashTransform`))
        (`self.StartSkill1Cooldown`)
        (`self.MulticastDisableMoveInput`)
        (`SceneComponent.SetVisibility` _knight_skill1_cone true true)
        (set `PrimitiveComponent.bGenerateOverlapEvents` true _knight_skill1_cone)
        (`Timeline|Dash_TL` :!via `PlayFromStart`
          (:`Update`
            (`PawnMovementComponent.AddInputVector` (`self.CharacterMovement`) (`self.DashDirection`) true))
          (:`Finished`
            (set `CharacterMovementComponent.MaxWalkSpeed` (+ (* (`KismetMathLibrary.Conv_IntToDouble` _player_struct_mv_spd) 1.0) 500.0) _charactermovement)
            (`self.MulticastSwordDashTransform` (`self.SwordOrigTransform`))
            (`self.MulticastEnableMoveInput`)
            (set `self.CanRotate` true)
            (set `self.IsDashing` false)
            (`SceneComponent.SetVisibility` _knight_skill1_cone_2 false true)
            (set `PrimitiveComponent.bGenerateOverlapEvents` false _knight_skill1_cone_2)
            (if (!= _returnvalue_2 null)
              (`Controller.SetIgnoreMoveInput` _returnvalue_2 false))))))))

(event `Handle Skill1Command Client`
  (`self.Handle Skill1Command Server`))

(event `self.HandleSkill1Command`
  (`/Engine/EditorBlueprintResources/ActorMacros.Switch Has Authority`
    (:`Authority`
      (if (`KismetSystemLibrary.IsServer`)
        (`self.Handle Skill1Command Server`)
        (else
          (`self.Handle Skill1Command Client` :!label _label))))
    (:`Remote`
      (goto _label))))

(event `StartSkill1Cooldown`
  (bind (_player_struct_hp _player_struct_hp_max _player_struct_cur _player_struct_inc _player_struct_lvl _player_struct_xp _player_struct_atk _player_struct_atk_spd _player_struct_mv_spd _player_struct_atk_size _player_struct_class _player_struct_cdr) (break `/Game/Characters/Player_Data_Struct` (`self.Player_Struct`)))
  (set `self.IsDashOnCooldown` true)
  (bind _returnvalue (`KismetSystemLibrary.K2_SetTimerDelegate` (delegate `OnSkill1CooldownEnd`) (/ 5.0 (+ (`KismetMathLibrary.Conv_IntToDouble` _player_struct_cdr) 1.0))))
  (set `self.Skill1Timer` _returnvalue))

(event `OnSkill1CooldownEnd`
  (set `self.IsDashOnCooldown` false))

(event `self.Knight_Skill1_Cone.OnComponentBeginOverlap`
  (params (OverlappedComponent :type "PrimitiveComponent Object Reference") (OtherActor :type "Actor Object Reference") (OtherComp :type "PrimitiveComponent Object Reference") (OtherBodyIndex :type Integer) (bFromSweep :type Boolean) (SweepResult :type "HitResult Structure (by ref)"))
  ;[1 1 1] Weapon Collision
  (if (!= (`GameplayStatics.GetObjectClass` OtherActor) (`GameplayStatics.GetObjectClass` self))
    (`/Engine/EditorBlueprintResources/ActorMacros.Switch Has Authority`
      (:`Authority`
        (if (`KismetSystemLibrary.IsServer`)
          (`self.ApplyDamageClient` OtherActor)
          (else
            (`self.ApplyDamageServer` OtherActor :!label _label_2))))
      (:`Remote`
        (goto _label_2)))))

(event `self.HandleSkill2Command`
  (`KismetSystemLibrary.PrintString` "Tambourine Club2!!"))

(event `self.HandleSkill3Command`
  (`KismetSystemLibrary.PrintString` "Tambourine Club3!!"))

(event `self.ReceiveTick`
  (params (DeltaSeconds :type "Float (single-precision)"))
  (`parent.ReceiveTick` DeltaSeconds)
  (`SceneComponent.K2_AddRelativeRotation` (`self.Knight_Skill1_Cone`) (struct :`Pitch` 1.0) false false))

(event `self.HandleSkill4Command`
  (`KismetSystemLibrary.PrintString` "Tambourine Club4!!"))

(event `Skill1TimerClient`
  (bind (_player_struct_hp _player_struct_hp_max _player_struct_cur _player_struct_inc _player_struct_lvl _player_struct_xp _player_struct_atk _player_struct_atk_spd _player_struct_mv_spd _player_struct_atk_size _player_struct_class _player_struct_cdr) (break `/Game/Characters/Player_Data_Struct` (`self.Player_Struct`)))
  (bind _returnvalue (`KismetSystemLibrary.K2_SetTimerDelegate` (delegate `OnSkill1LocalTimerEnd`) (/ 5.0 (+ (`KismetMathLibrary.Conv_IntToDouble` _player_struct_cdr) 1.0))))
  (set `self.Skill1Timer_Client` _returnvalue))

(event `OnSkill1LocalTimerEnd`)

(fn `StartLocalSkill1Timer`
  (`parent.StartLocalSkill1Timer`)
  (`/Engine/EditorBlueprintResources/ActorMacros.Switch Has Authority`
    (:`Authority`
      (`self.Skill1TimerClient`))))

(fn `UserConstructionScript`
  (`parent.UserConstructionScript`))