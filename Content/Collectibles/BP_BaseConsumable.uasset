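; Base collectible pawn with an animated sprite that homes in on the player and grants an "XP1" consumable.
; A random delay staggers sprite playback, and sphere overlap with a player character starts an AI MoveTo chase after a brief pause.
; Success calls CollectConsumable on the player and destroys the pickup; failure polls until the player is at least 50 units away, then chases again.
; Random launch velocity and impulse nodes are left unconnected.
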(event `self.ReceiveBeginPlay`
  (bind _sprite (`self.Sprite`))
  (`PaperFlipbookComponent.Stop` _sprite)
  (`KismetSystemLibrary.Delay` (`KismetMathLibrary.RandomFloatInRange` 0.0 1.0))
  (`PaperFlipbookComponent.PlayFromStart` _sprite))

(event `TrackPlayer`
  (params (Player :type "/Game/Characters/BP_BasePlayerCharacter Object Reference"))
  (`KismetSystemLibrary.Delay` 0.2)
  (if (>= (`self.GetDistanceTo` Player self) 50.0)
    (`self.ChasePlayer` Player)
    (else
      (`self.TrackPlayer` Player))))

(event `ChasePlayer`
  (params (Actor :type "/Game/Characters/BP_BasePlayerCharacter Object Reference"))
  (set `self.IsBeingCollected` true)
  (`|AIMoveTo` self (0.0 0.0 0.0) Actor 0.001
    (:`OnSuccess`
      (`/Game/Characters/BP_BasePlayerCharacter.CollectConsumable` Actor "XP1")
      (`self.K2_DestroyActor`))
    (:`OnFail`
      (`KismetSystemLibrary.Delay` 0.1)
      (`self.TrackPlayer` Actor))))

(event `self.Sphere.OnComponentBeginOverlap`
  (params (OverlappedComponent :type "PrimitiveComponent Object Reference") (OtherActor :type "Actor Object Reference") (OtherComp :type "PrimitiveComponent Object Reference") (OtherBodyIndex :type Integer) (bFromSweep :type Boolean) (SweepResult :type "HitResult Structure (by ref)"))
  (if (`KismetMathLibrary.ClassIsChildOf` (`GameplayStatics.GetObjectClass` OtherActor) "/Game/Characters/BP_BasePlayerCharacter.BP_BasePlayerCharacter_C")
    (bind _asbp_base_player_character (cast `/Game/Characters/BP_BasePlayerCharacter` OtherActor))
    (`KismetSystemLibrary.Delay` 0.1)
    (`self.ChasePlayer` _asbp_base_player_character)))

(fn `UserConstructionScript`)