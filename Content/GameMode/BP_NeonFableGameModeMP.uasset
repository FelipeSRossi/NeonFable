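; Multiplayer game mode for Neon Fable that assigns joining players a number and team and spawns their knight characters.
; On login it finds the game controller, sorts PlayerStarts into two team lists by tag and triggers team selection on the player state.
; A separate ContinuePostLogin event respawns the player at the team's next start, then registers them with the game controller.
; Respawning destroys any existing pawn and possesses a new knight.
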(event `RespawnPlayer`
  (params (PlayerController :type "/Game/TopDown/Blueprints/BP_TopDownPlayerController Object Reference"))
  (bind _returnvalue (`Controller.K2_GetPawn` PlayerController))
  (bind _asbp_neon_fable_player_state_mp (cast `/Game/GameMode/BP_NeonFablePlayerStateMP` (`Controller.PlayerState` PlayerController)))
  (`/Engine/EditorBlueprintResources/StandardMacros.IsValid` _returnvalue
    (:`Is Valid`
      (`self.K2_DestroyActor` _returnvalue))
    (:`Is Not Valid`
      _))
  (switch `int` (`/Game/GameMode/BP_NeonFablePlayerStateMP.TeamNumber` _asbp_neon_fable_player_state_mp)
    (:`0`
      (bind _returnvalue_2 (`|SpawnActorFromClass` "/Game/Characters/Knight/BP_KnightCharacter.BP_KnightCharacter_C" (`self.GetTransform` (`|GetArrayItem` (`self.TeamStart1`) (`self.Team1Pointer`))) "AdjustIfPossibleButAlwaysSpawn" "OverrideRootScale" null null))
      (set `/Game/Characters/BP_BasePlayerCharacter.TeamNumber` 0 _returnvalue_2)
      (`Controller.Possess` PlayerController _returnvalue_2)
      (`/Engine/EditorBlueprintResources/StandardMacros.IncrementInt` (`self.Team1Pointer`)
        (:`  `
          (set `/Game/TopDown/Blueprints/BP_TopDownPlayerController.PlayerPawn` _returnvalue_2 PlayerController))))
    (:`1`
      (bind _returnvalue_3 (`|SpawnActorFromClass` "/Game/Characters/Knight/BP_KnightCharacter.BP_KnightCharacter_C" (`self.GetTransform` (`|GetArrayItem` (`self.TeamStart2`) (`self.Team2Pointer`))) "AdjustIfPossibleButAlwaysSpawn" "OverrideRootScale" null null))
      (set `/Game/Characters/BP_BasePlayerCharacter.TeamNumber` 1 _returnvalue_3)
      (`Controller.Possess` PlayerController _returnvalue_3)
      (`/Engine/EditorBlueprintResources/StandardMacros.IncrementInt` (`self.Team2Pointer`)
        (:`  `
          (set `/Game/TopDown/Blueprints/BP_TopDownPlayerController.PlayerPawn` _returnvalue_3 PlayerController))))))

(event `self.K2_PostLogin`
  (params (NewPlayer :type "PlayerController Object Reference"))
  ;[1 1 1] On Post Login
  (`/Engine/EditorBlueprintResources/StandardMacros.IsValid` (`self.GameController`)
    (:`Is Valid`
      (`/Engine/EditorBlueprintResources/ActorMacros.Switch Has Authority` :!label _label
        (:`Authority`
          (if (== (+ (`KismetArrayLibrary.Array_Length` (`self.TeamStart1`)) (`KismetArrayLibrary.Array_Length` (`self.TeamStart2`))) 0)
            (bind _outactors (`GameplayStatics.GetAllActorsOfClass` "/Script/Engine.PlayerStart"))
            (for _array_element _outactors
              (if (== (`PlayerStart.PlayerStartTag` _array_element) "Team2")
                (`KismetArrayLibrary.Array_AddUnique` (`self.TeamStart2`) _array_element)
                (else
                  (`KismetArrayLibrary.Array_AddUnique` (`self.TeamStart1`) _array_element)))))
          (bind _asbp_neon_fable_player_state_mp (cast `/Game/GameMode/BP_NeonFablePlayerStateMP` (`Controller.PlayerState` NewPlayer)))
          (set `/Game/GameMode/BP_NeonFablePlayerStateMP.PlayerNumber` (- (`KismetArrayLibrary.Array_Length` (`GameStateBase.PlayerArray` (`GameplayStatics.GetGameState`))) 1) _asbp_neon_fable_player_state_mp)
          (`/Game/GameMode/BP_NeonFablePlayerStateMP.Set Chosen Team` _asbp_neon_fable_player_state_mp))))
    (:`Is Not Valid`
      (bind _found (`self.GetGameController`))
      (if _found
        (goto _label)))))

(event `ContinuePostLogin`
  ;[1 1 1] On Post Login
  (bind _asbp_top_down_player_controller (cast `/Game/TopDown/Blueprints/BP_TopDownPlayerController` (stale `self.K2_PostLogin` NewPlayer)))
  (`self.RespawnPlayer` _asbp_top_down_player_controller)
  (`/Game/TopDown/Blueprints/BP_TopDownPlayerController.ClientPostLogin` _asbp_top_down_player_controller)
  (`/Game/GameMode/BP_NeonFableGameControllerMP.AddPlayer` (`self.GameController`) _asbp_top_down_player_controller))

(fn `GetGameController`
  (returns (Found :type Boolean))
  (bind _outactors (`GameplayStatics.GetAllActorsOfClass` "/Game/GameMode/BP_NeonFableGameControllerMP.BP_NeonFableGameControllerMP_C"))
  (bind _output (`|GetArrayItem` _outactors))
  (`/Engine/EditorBlueprintResources/StandardMacros.IsValid` _output
    (:`Is Valid`
      (set `self.GameController` _output)
      (return true))
    (:`Is Not Valid`
      (return false))))

(fn `OnRep_TeamStart1`)

(fn `UserConstructionScript`)