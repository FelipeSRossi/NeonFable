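; Multiplayer game instance for NeonFable that hosts and joins sessions and manages front-end screens from startup into gameplay.
; A TransitionToState macro drives a state machine that hides the outgoing widget or destroys the session when leaving gameplay, while callers lazily create and cache each screen.
; Host opens the map as a listen server, with LAN optional.
; Session failures, travel errors and client-side network errors open an error dialog that destroys the session.
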(event `JoinGame`
  (params (GameToJoin :type "BlueprintSessionResult Structure"))
  ;[1 1 1] Join Game
  (`self.ShowLoadingScreen`)
  (`JoinSessionCallbackProxy.JoinSession` (`GameplayStatics.GetPlayerController` 0) GameToJoin
    (:`OnFailure`
      (`self.DisplayErrorDialog` "FAILED TO JOIN"))))

(event `HostGame`
  ;[1 1 1] Host Game
  (`self.ShowLoadingScreen`)
  (`CreateSessionCallbackProxy.CreateSession` (`GameplayStatics.GetPlayerController` 0) 4 (`self.EnableLan`)
    (:`OnSuccess`
      (`GameplayStatics.OpenLevel` "NeonFableMap_1" true "listen"))
    (:`OnFailure`
      (`self.DisplayErrorDialog` "FAILED! NO SESSION CREATED"))))

(event `ShowServers`
  (bind _returnvalue (`GameplayStatics.GetPlayerController` 0))
  (bind _serverlist (`self.ServerList`))
  ;[1 1 1] Show Servers
  (`self.TransitionToState` "NewEnumerator2"
    (:`NewState`
      (`/Engine/EditorBlueprintResources/StandardMacros.IsValid` (`self.ServerList`)
        (:`Is Valid`
          _)
        (:`Is Not Valid`
          (bind _returnvalue_2 (`|CreateWidget` "/Game/UI/BP_UI_ServerList.BP_UI_ServerList_C" _returnvalue))
          (set `self.ServerList` _returnvalue_2)))
      (`UserWidget.AddToViewport` _serverlist 0)
      (`WidgetBlueprintLibrary.SetInputMode_UIOnlyEx` _returnvalue _serverlist))))

(event `ShowMainMenu`
  (bind _returnvalue (`GameplayStatics.GetPlayerController` 0))
  ;[1 1 1] Show Main Menu
  (`self.IsCurrentState` "NewEnumerator5"
    (:`True`
      (`GameplayStatics.OpenLevel` "StartMenu")
      (`KismetSystemLibrary.Delay` 0.2))
    (:`False`
      _))
  (`self.TransitionToState` "NewEnumerator1"
    (:`NewState`
      (`/Engine/EditorBlueprintResources/StandardMacros.IsValid` (`self.MainMenu`)
        (:`Is Valid`
          _)
        (:`Is Not Valid`
          (bind _returnvalue_2 (`|CreateWidget` "/Game/UI/BP_UI_Main.BP_UI_Main_C" (`GameplayStatics.GetPlayerController` 0)))
          (bind _output_get (set `self.MainMenu` _returnvalue_2))))
      (`WidgetBlueprintLibrary.SetInputMode_UIOnlyEx` _returnvalue _output_get)
      (`UserWidget.AddToViewport` (`self.MainMenu`) 0)
      (set `PlayerController.bShowMouseCursor` true _returnvalue))))

(event `TravelError`
  (params (FailureType :type "ETravelFailure Enum" :default "NoLevel"))
  (`self.DisplayErrorDialog` (`|GetEnumeratorNameAsString` FailureType)))

(event `NetworkError`
  (params (FailureType :type "ENetworkFailure Enum" :default "NetDriverAlreadyExists") (IsServer :type Boolean))
  (if (not IsServer)
    (`self.DisplayErrorDialog` (`|GetEnumeratorNameAsString` FailureType))))

(event `DestroySessionCaller`
  ;[1 1 1] Destroy Session Caller
  (`DestroySessionCallbackProxy.DestroySession` (`GameplayStatics.GetPlayerController` 0)))

(event `ShowLoadingScreen`
  (bind _returnvalue (`GameplayStatics.GetPlayerController` 0))
  (bind _loadingscreen (`self.LoadingScreen`))
  ;[1 1 1] Show Loading Screen
  (`self.TransitionToState` "NewEnumerator3"
    (:`NewState`
      (`/Engine/EditorBlueprintResources/StandardMacros.IsValid` (`self.LoadingScreen`)
        (:`Is Valid`
          _)
        (:`Is Not Valid`
          (bind _returnvalue_2 (`|CreateWidget` "/Game/UI/BP_UI_LoadingScreen.BP_UI_LoadingScreen_C" _returnvalue))
          (set `self.LoadingScreen` _returnvalue_2)))
      (`UserWidget.AddToViewport` _loadingscreen 0)
      (`WidgetBlueprintLibrary.SetInputMode_UIOnlyEx` _returnvalue _loadingscreen))))

(fn `BeginPlayShowMainMenu`
  (`self.IsCurrentState` "NewEnumerator0"
    (:`True`
      (`self.ShowMainMenu `))))

(fn `GetTeamNumber`
  (returns (TeamNumber :type Integer))
  (return (`self.TeamNumber`)))

(fn `HideWidget`
  (params (Widget :type "Widget Object Reference"))
  (`Widget.RemoveFromParent` Widget))

(fn `NetErrorToString`
  (params (`In Error` :type "ENetworkFailure Enum" :default "NetDriverAlreadyExists"))
  (returns (OutString :type String))
  (locals (ErrorString :type String))
  (switch `ENetworkFailure` `In Error`
    (:`NetDriverAlreadyExists`
      (set `local.ErrorString` "ERROR: CONNECTION LOST" :!label _label))
    (:`NetDriverCreateFailure`
      (goto _label))
    (:`NetDriverListenFailure`
      (goto _label))
    (:`ConnectionLost`
      (goto _label))
    (:`ConnectionTimeout`
      (set `local.ErrorString` "ERROR: CONNECTION TIMED OUT"))
    (:`FailureReceived`
      (goto _label))
    (:`OutdatedClient`
      (goto _label))
    (:`OutdatedServer`
      (goto _label))
    (:`PendingConnectionFailure`
      (goto _label)))
  (return (`local.ErrorString`)))

(fn `StartPlayingState`
  (`self.TransitionToState` "NewEnumerator5"))

(fn `TravelToErrorString`
  (params (InError :type "ETravelFailure Enum" :default "NoLevel"))
  (returns (OutString :type String))
  (return (`KismetStringLibrary.Concat_StrStr` "ERROR: TRAVEL FAILURE" (`|GetEnumeratorNameAsString` InError))))