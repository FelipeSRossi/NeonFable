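; Multiplayer player state for Neon Fable that carries the player's chosen team number to the server during login.
; SetChosenTeam reads the team number stored in the game instance and passes it to a server event.
; The server stores it in TeamNumber, then tells the multiplayer game mode to continue its post-login flow.
; TeamNumber has a RepNotify function, which is currently empty.
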(event `Set Chosen Team`
  (bind _teamnumber (`self.GetChosenTeamNumber`))
  (`self.SERVER_SetTeamNumber` _teamnumber))

(event `SERVER_SetTeamNumber`
  (params (TeamNumber :type Integer))
  (set `self.TeamNumber` TeamNumber)
  (bind _asbp_neon_fable_game_mode_mp (cast `/Game/GameMode/BP_NeonFableGameModeMP` (`GameplayStatics.GetGameMode`)))
  (`/Game/GameMode/BP_NeonFableGameModeMP.ContinuePostLogin` _asbp_neon_fable_game_mode_mp))

(fn `GetChosenTeamNumber`
  (returns (TeamNumber :type Integer))
  (bind _asbp_neon_fable_game_instance_mp (cast `/Game/GameMode/BP_NeonFableGameInstanceMP` (`GameplayStatics.GetGameInstance`)))
  (return (`/Game/GameMode/BP_NeonFableGameInstanceMP.TeamNumber` _asbp_neon_fable_game_instance_mp)))

(fn `OnRep_TeamNumber`)

(fn `UserConstructionScript`)