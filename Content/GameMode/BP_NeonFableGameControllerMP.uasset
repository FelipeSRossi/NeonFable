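; Multiplayer game controller for Neon Fable that registers players and sorts their pawns by team.
; AddPlayer casts to the player controller and state, then inserts both into arrays at the state's non-negative PlayerNumber, only printing a notice if a valid state already occupies that index.
; It then copies that number onto the controlled character and adds it to Team1Pawns for team zero, otherwise Team2Pawns.
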(event `AddPlayer`
  (params (NewPlayer :type "PlayerController Object Reference"))
  (bind _playerstates (`self.PlayerStates`))
  (bind _asbp_top_down_player_controller (cast `/Game/TopDown/Blueprints/BP_TopDownPlayerController` NewPlayer))
  (bind _asbp_neon_fable_player_state_mp (cast `/Game/GameMode/BP_NeonFablePlayerStateMP` (`Controller.PlayerState` _asbp_top_down_player_controller)))
  (bind _playernumber (`/Game/GameMode/BP_NeonFablePlayerStateMP.PlayerNumber` _asbp_neon_fable_player_state_mp))
  (if (>= _playernumber 0)
    (if (`KismetArrayLibrary.Array_IsValidIndex` _playerstates _playernumber)
      (`/Engine/EditorBlueprintResources/StandardMacros.IsValid` (`|GetArrayItem` _playerstates _playernumber)
        (:`Is Valid`
          (`KismetSystemLibrary.PrintString` "EXISTS ALREADY"))
        (:`Is Not Valid`
          (`KismetArrayLibrary.Array_Insert` (`self.PlayerStates`) _asbp_neon_fable_player_state_mp _playernumber :!label _label)
          (`KismetArrayLibrary.Array_Insert` (`self.PlayerControllers`) _asbp_top_down_player_controller _playernumber)
          (bind _asbp_base_player_character (cast `/Game/Characters/BP_BasePlayerCharacter` (`Controller.K2_GetPawn` _asbp_top_down_player_controller)))
          (set `/Game/Characters/BP_BasePlayerCharacter.PlayerNumber` _playernumber _asbp_base_player_character)
          (if (== (`/Game/Characters/BP_BasePlayerCharacter.TeamNumber` _asbp_base_player_character) 0)
            (`KismetArrayLibrary.Array_Add` (`self.Team1Pawns`) _asbp_base_player_character)
            (else
              (`KismetArrayLibrary.Array_Add` (`self.Team2Pawns`) _asbp_base_player_character)))))
      (else
        (goto _label)))))

(fn `UserConstructionScript`)