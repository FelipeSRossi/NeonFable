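; BP_LensFlare is an actor that renders a lens flare through a post process material.
; Construction creates a dynamic instance of the chosen material, feeds it the actor's location and forward vector plus the sphere radius as max draw distance, then assigns it to the PostProcess component.
; Tick refreshes location and direction, and runs only when the sphere is Movable.
; Toggle and set functions switch the post process on or off.
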(event `self.ReceiveBeginPlay`
  (`self.SetActorTickEnabled` (`|EnumEquality` (`SceneComponent.Mobility` (`self.Sphere`)) "Movable")))

(event `self.ReceiveTick`
  (params (DeltaSeconds :type "Float (single-precision)"))
  (`self.Update Material Parameters`))

(fn `Initialize`
  (locals (`L Post Process Settings` :type "PostProcessSettings Structure"))
  (`self.Material`
    (:`then`
      (set `local.L Post Process Settings` (`PostProcessComponent.Settings` (`self.PostProcess`)))
      (bind _returnvalue (`KismetMaterialLibrary.CreateDynamicMaterialInstance` (`self.Material`)))
      (bind _output_get (set `self.Flare MID` _returnvalue))
      (`MaterialInstanceDynamic.SetVectorParameterValue` _output_get "Location" (`KismetMathLibrary.Conv_VectorToLinearColor` (`self.K2_GetActorLocation`)))
      (`MaterialInstanceDynamic.SetVectorParameterValue` (`self.Flare MID`) "Direction" (`KismetMathLibrary.Conv_VectorToLinearColor` (`self.GetActorForwardVector`)))
      (`MaterialInstanceDynamic.SetScalarParameterValue` (`self.Flare MID`) "Max Draw Distance" (`SphereComponent.GetScaledSphereRadius` (`self.Sphere`)))
      (bind _structout (setmembers `PostProcessSettings` :`StructRef` (`local.L Post Process Settings`) :`WeightedBlendables` (make `WeightedBlendables` (`|MakeArray` (make `WeightedBlendable` 1.0 (`self.Flare MID`)) :!type "WeightedBlendable Structure"))))
      (set `PostProcessComponent.Settings` _structout (`self.PostProcess`))
      (return))
    (:`else`
      (`KismetSystemLibrary.PrintString` "Error: Invalid material!" true true (struct :`R` 1.0 :`A` 1.0) 3.0)
      (return))))

(fn `Set Enabled`
  (params (Enabled :type Boolean))
  (bind _output_get (set `PostProcessComponent.bEnabled` Enabled (`self.PostProcess`)))
  (if _output_get
    (`self.Update Material Parameters`))
  (return))

(fn `Toggle Enabled`
  (bind _postprocess (`self.PostProcess`))
  (set `PostProcessComponent.bEnabled` (not (`PostProcessComponent.bEnabled` _postprocess)) _postprocess)
  (`self.Update Material Parameters`)
  (return))

(fn `Update Material Parameters`
  (`MaterialInstanceDynamic.SetVectorParameterValue` (`self.Flare MID`) "Location" (`KismetMathLibrary.Conv_VectorToLinearColor` (`self.K2_GetActorLocation`)))
  (`MaterialInstanceDynamic.SetVectorParameterValue` (`self.Flare MID`) "Direction" (`KismetMathLibrary.Conv_VectorToLinearColor` (`self.GetActorForwardVector`)))
  (return))

(fn `UserConstructionScript`
  (`self.Initialize`)
  (`SceneComponent.SetVisibility` (`self.Sphere`) (`self.Show Sphere`) false))